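; Player bird pawn for a Flappy Bird-style game, driven by physics on a capsule with sprite swaps for jumping and death.
; It hovers until the first Jump press enables gravity, and each press resets velocity before applying upward force.
; While rising, Tick applies a downforce chosen by jump input to vary jump height.
; Overlapping an enemy-tagged component kills and spins the bird, then loads the opening level; AddPoint increments and prints score.
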(event OnComponentBeginOverlap(Capsule)
  (params (OverlappedComponent :type Primitive%20Component%20Object%20Reference) (OtherActor :type Actor%20Object%20Reference) (OtherComp :type Primitive%20Component%20Object%20Reference) (OtherBodyIndex :type Integer) (bFromSweep :type Boolean) (SweepResult :type Hit%20Result%20Structure%20%28by%20ref%29))
  ;[1 1 1] When Capsule hits other object, kill bird and load opening level
  (Utilities|IsValid OtherComp
    (:Is%20Valid
      (if (Components|ComponentHasTag OtherComp (Variables|Default|GetEnemyTag))
        (if (Variables|BirdStatus|GetisAlive)
          (BirdStatus|KillBird)
          (Rendering|Components|Sprite|SetSprite (Variables|Default|GetBird) (Variables|BirdStatus|GetDeathSprite))
          ;;[1 1 1] Maybe Make this a seperate thing? (bird video #3 @ 9:00)
          (Utilities|FlowControl|Delay 3.0)
          (Game|OpenLevel(byObjectReference) "/Game/Levels/Opening_Level.Opening_Level"))))))

(event EventBeginPlay
  ;[1 1 1] Hover Mechanic when starting
  (Physics|SetEnableGravity (Variables|Default|GetCapsule) false))

(event EventTick
  (params (DeltaSeconds :type Float%20%28single-precision%29))
  ;[1 1 1] Downforce Gravity Setting and Long vs Short Jump setting. To Change Player Jump Height/Power on long/short click, change appropriate variables
  (bind _returnvalue (Physics|GetPhysicsLinearVelocity (Variables|Default|GetCapsule) "None"))
  (if (> (.z _returnvalue) 0.0)
    (if (== (Input|AxisValues|GetJump) 1.0)
      (Variables|JumpControls|SetDownforce (* (Variables|JumpControls|GetShort%20Click%20Downforce) DeltaSeconds))
      (else
        (Variables|JumpControls|SetDownforce (* (Variables|JumpControls|GetLong%20Click%20Downforce) DeltaSeconds))))
    (Physics|AddForce (Variables|Default|GetCapsule) (Math|Vector|MakeVector 0.0 0.0 (Variables|JumpControls|GetDownforce)) "None" false)))

(event Input|ActionEvents|InputActionJump
  (params (Key :type Key%20Structure :default "None"))
  ;[1 1 1] Jump Controls
  (:Pressed
    (if (Variables|BirdStatus|GetisPlaying)
      _
      (else
        (Variables|BirdStatus|SetisPlaying true)
        (Physics|SetEnableGravity (Variables|Default|GetCapsule) true)))
    (if (Variables|BirdStatus|GetisAlive)
      (JumpControls|Jump))))

(event Input|ActionEvents|InputActionJump
  (params (Key :type Key%20Structure :default "None"))
  ;[1 1 1] Animation for 2 Sprites, Add Sound Effects here (But later)
  (:Pressed
    (if (Variables|BirdStatus|GetisAlive)
      (Rendering|Components|Sprite|SetSprite (Variables|Default|GetBird) (Variables|BirdStatus|GetSecondSprite))))
  (:Released
    (if (Variables|BirdStatus|GetisAlive)
      (Utilities|FlowControl|Delay 0.1)
      (Rendering|Components|Sprite|SetSprite (Variables|Default|GetBird) (Variables|BirdStatus|GetFirstSprite)))))

(fn ConstructionScript)

(fn Jump
  (Physics|SetPhysicsLinearVelocity (Variables|Default|GetCapsule) "0, 0, 0" false "None")
  (Physics|AddForce (Variables|Default|GetCapsule) (Math|Vector|MakeVector 0.0 0.0 (Variables|JumpControls|GetJump%20Force)) "None" false))

(fn KillBird
  (Variables|BirdStatus|SetisAlive false)
  (JumpControls|Jump)
  (Class|PrimitiveComponent|AddTorqueinDegrees (Variables|Default|GetCapsule) "0,100000000.000000, 0" "None" false))

(fn AddPoint
  (bind _result (Math|Integer|IncrementInt (Variables|Default|GetScore))
    (:%20%20
      (Development|PrintString (Utilities|String|ToString(Integer) _result)))))