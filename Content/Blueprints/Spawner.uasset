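; Spawner actor that produces Pipe obstacles at its own transform while the player's bird is playing.
; BeginPlay caches the player pawn as a BirdController, printing an error if the cast fails.
; Tick checks that pawn's IsPlaying flag and runs into a Delay before spawning, so the latent node throttles per-frame calls into a fixed spawn interval.
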(event EventBeginPlay
  (bind _asbird_controller (Utilities|Casting|CastToBirdController (Game|Player|GetPlayerPawn 0))
    (:then
      (Variables|Default|SetPlayerRef _asbird_controller))
    (:CastFailed
      (Development|PrintString "Error, Cast to BirdController Fialed"))))

(event EventTick
  (params (DeltaSeconds :type Float%20%28single-precision%29))
  (if (Variables|/Game/Blueprints/BirdController.BirdController_C|GetisPlaying (Variables|Default|GetPlayerRef))
    (Utilities|FlowControl|Delay 1.5)
    (Game|SpawnActorfromClass "/Game/Blueprints/Pipe.Pipe_C" (Transformation|GetWorldTransform (Variables|Default|GetDefaultSceneRoot)) "Undefined" 0 0)))

(fn ConstructionScript)